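; BP_Projectile is a player-related projectile that destroys enemies on contact and awards score.
; Each tick it moves along world X, then resets its speed to the player's forward speed plus a fixed boost.
; A box overlap with BP_Enemy destroys both actors and increments the player's score and score widget.
; Overlapping a BP_Healthpack destroys only the projectile.
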(event `self.ReceiveTick`
  (params (DeltaSeconds :type "Float (single-precision)"))
  (`self.K2_AddActorWorldOffset` (`KismetMathLibrary.MakeVector` (* DeltaSeconds (`self.ForwardSpeed`))))
  (`self.UpdateSpeed`))

(event `self.Box.OnComponentBeginOverlap`
  (params (OverlappedComponent :type "PrimitiveComponent Object Reference") (OtherActor :type "Actor Object Reference") (OtherComp :type "PrimitiveComponent Object Reference") (OtherBodyIndex :type Integer) (bFromSweep :type Boolean) (SweepResult :type "HitResult Structure (by ref)"))
  (bind _asbp_enemy (cast `/Game/InfiniteMatrix/Blueprints/BP_Enemy` OtherActor)
    (:`then`
      (`self.K2_DestroyActor` _asbp_enemy)
      (`self.K2_DestroyActor`)
      (bind _asbp_player (cast `/Game/InfiniteMatrix/Blueprints/BP_Player` (`GameplayStatics.GetPlayerPawn` 0)))
      (`/Engine/EditorBlueprintResources/StandardMacros.IncrementInt` (`/Game/InfiniteMatrix/Blueprints/BP_Player.Score` _asbp_player)
        (:`  `
          (`/Game/InfiniteMatrix/UI/WBP_Score.IncrementScore` (`/Game/InfiniteMatrix/Blueprints/BP_Player.WB_Score` _asbp_player)))))
    (:`CastFailed`
      (cast `/Game/InfiniteMatrix/Blueprints/BP_Healthpack` OtherActor)
      (`self.K2_DestroyActor`))))

(fn `UpdateSpeed`
  (bind _asbp_player (cast `/Game/InfiniteMatrix/Blueprints/BP_Player` (`GameplayStatics.GetPlayerPawn` 0)))
  (set `self.ForwardSpeed` (+ (`/Game/InfiniteMatrix/Blueprints/BP_Player.ForwardSpeed` _asbp_player) 1500.0)))

(fn `UserConstructionScript`)