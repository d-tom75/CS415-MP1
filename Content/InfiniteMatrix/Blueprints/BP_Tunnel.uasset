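; BP_Tunnel is an endless-tunnel segment with a spinning holed wall that damages BP_Player on contact and triggers restart at zero health.
; Entering TriggerZone makes TunnelSpawner spawn another tunnel, destroys this one and increments player score.
; TriggerZone end overlap increments the score widget if no wall was hit and scores differ.
; Randomize functions, not called here, vary wall mesh and roll, occasionally spawn healthpacks, and spawn enemies within SpawnArea.
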(event `self.ReceiveTick`
  (params (DeltaSeconds :type "Float (single-precision)"))
  (`SceneComponent.K2_AddLocalRotation` (`self.WallMesh`) (`KismetMathLibrary.MakeRotator` (* DeltaSeconds (`self.RotateSpeed`))) false false))

(event `self.TriggerZone.OnComponentBeginOverlap`
  (params (OverlappedComponent :type "PrimitiveComponent Object Reference") (OtherActor :type "Actor Object Reference") (OtherComp :type "PrimitiveComponent Object Reference") (OtherBodyIndex :type Integer) (bFromSweep :type Boolean) (SweepResult :type "HitResult Structure (by ref)"))
  (bind _asbp_player (cast `/Game/InfiniteMatrix/Blueprints/BP_Player` OtherActor))
  (`/Game/InfiniteMatrix/Blueprints/BP_TunnelSpawner.SpawnTunnelAtSpawnPoint` (`self.TunnelSpawner`))
  (`self.K2_DestroyActor`)
  (bind _result (`/Engine/EditorBlueprintResources/StandardMacros.IncrementInt` (`/Game/InfiniteMatrix/Blueprints/BP_Player.Score` _asbp_player))
    (:`  `
      (bind _output_get (set `/Game/InfiniteMatrix/Blueprints/BP_Player.Score` _result _asbp_player))
      (`KismetSystemLibrary.PrintText` (`KismetTextLibrary.Conv_IntToText` _output_get)))))

(event `self.TriggerZone.OnComponentEndOverlap`
  (params (OverlappedComponent :type "PrimitiveComponent Object Reference") (OtherActor :type "Actor Object Reference") (OtherComp :type "PrimitiveComponent Object Reference") (OtherBodyIndex :type Integer))
  (bind _asbp_player (cast `/Game/InfiniteMatrix/Blueprints/BP_Player` OtherActor))
  (if (`self.HitObstacle`)
    (set `self.HitObstacle` false)
    (else
      (set `self.HitObstacle` false)
      (bind _wb_score (`/Game/InfiniteMatrix/Blueprints/BP_Player.WB_Score` _asbp_player))
      (if (!= (`/Game/InfiniteMatrix/UI/WBP_Score.Score` _wb_score) (`/Game/InfiniteMatrix/Blueprints/BP_Player.Score` _asbp_player))
        (`/Game/InfiniteMatrix/UI/WBP_Score.IncrementScore` _wb_score)
        (`KismetSystemLibrary.PrintText` (`KismetTextLibrary.Conv_IntToText` (`/Game/InfiniteMatrix/UI/WBP_Score.Score` (`/Game/InfiniteMatrix/Blueprints/BP_Player.WB_Score` _asbp_player))))))))

(event `self.WallMesh.OnComponentBeginOverlap`
  (params (OverlappedComponent :type "PrimitiveComponent Object Reference") (OtherActor :type "Actor Object Reference") (OtherComp :type "PrimitiveComponent Object Reference") (OtherBodyIndex :type Integer) (bFromSweep :type Boolean) (SweepResult :type "HitResult Structure (by ref)"))
  (bind _asbp_player (cast `/Game/InfiniteMatrix/Blueprints/BP_Player` OtherActor))
  (set `self.HitObstacle` true)
  (bind _output_get (set `/Game/InfiniteMatrix/Blueprints/BP_Player.Health` (- (`/Game/InfiniteMatrix/Blueprints/BP_Player.Health` _asbp_player) 20.0) _asbp_player))
  (`/Game/InfiniteMatrix/UI/WBP_Healthbar.UpdateHealthbar` (`/Game/InfiniteMatrix/Blueprints/BP_Player.WB_Healthbar` _asbp_player) _output_get)
  (if (<= (`/Game/InfiniteMatrix/Blueprints/BP_Player.Health` _asbp_player) 0.0)
    (set `/Game/InfiniteMatrix/Blueprints/BP_Player.IsDead` true _asbp_player)
    (`/Game/InfiniteMatrix/Blueprints/BP_Player.DisplayRestart` _asbp_player)))

(fn `RandomizeEnemy`
  (bind (_origin _boxextent) (`KismetSystemLibrary.GetComponentBounds` (`self.SpawnArea`)))
  (`|SpawnActorFromClass` "/Game/InfiniteMatrix/Blueprints/BP_Enemy.BP_Enemy_C" (`KismetMathLibrary.Conv_VectorToTransform` (`KismetMathLibrary.RandomPointInBoundingBox` _origin _boxextent)) "DontSpawnIfColliding" "MultiplyWithRoot" null null))

(fn `RandomizeHealthpack`
  (bind (_origin _boxextent) (`KismetSystemLibrary.GetComponentBounds` (`self.SpawnArea`)))
  (bind (_returnvalue_location _returnvalue_rotation _returnvalue_scale) (`KismetMathLibrary.BreakTransform` (`KismetMathLibrary.Conv_VectorToTransform` (`KismetMathLibrary.RandomPointInBoundingBox` _origin _boxextent))))
  (if (== (`KismetMathLibrary.RandomIntegerInRange` 0 9) 0)
    (`|SpawnActorFromClass` "/Game/InfiniteMatrix/Blueprints/BP_Healthpack.BP_Healthpack_C" (`KismetMathLibrary.MakeTransform` _returnvalue_location (struct :`Pitch` 90.0) _returnvalue_scale) "DontSpawnIfColliding" "MultiplyWithRoot" null null)))

(fn `RandomizeWall`
  (`StaticMeshComponent.SetStaticMesh` (`self.WallMesh`) (select `int` (`KismetMathLibrary.RandomIntegerInRange` 0 3) :`0` "/Game/InfiniteMatrix/Meshes/SM_Hole_01.SM_Hole_01" :`1` "/Game/InfiniteMatrix/Meshes/SM_Hole_02.SM_Hole_02" :`2` "/Game/InfiniteMatrix/Meshes/SM_Hole_03.SM_Hole_03" :`3` "/Game/InfiniteMatrix/Meshes/SM_Hole_04.SM_Hole_04" :!type "StaticMesh Object Reference"))
  (`SceneComponent.K2_AddLocalRotation` (`self.WallMesh`) (`KismetMathLibrary.MakeRotator` (`KismetMathLibrary.RandomFloatInRange` 0.0 360.0)) false false))

(fn `UserConstructionScript`)