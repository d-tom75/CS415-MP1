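; BP_Healthpack is a health pickup that restores the player's health when the player overlaps it.
; On overlap it casts to BP_Player, adds a fixed amount of health capped at the maximum, and pushes the new value to the player's WBHealthbar widget.
; The pack then destroys itself, even if the player was already at full health.
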(event `self.ReceiveActorBeginOverlap`
  (params (OtherActor :type "Actor Object Reference"))
  (bind _asbp_player (cast `/Game/InfiniteMatrix/Blueprints/BP_Player` OtherActor))
  (if (<= (`/Game/InfiniteMatrix/Blueprints/BP_Player.Health` _asbp_player) 80.0)
    (bind _output_get (set `/Game/InfiniteMatrix/Blueprints/BP_Player.Health` (+ (`/Game/InfiniteMatrix/Blueprints/BP_Player.Health` _asbp_player) 20.0) _asbp_player))
    (bind _wb_healthbar (`/Game/InfiniteMatrix/Blueprints/BP_Player.WB_Healthbar` _asbp_player))
    (`/Game/InfiniteMatrix/UI/WBP_Healthbar.UpdateHealthbar` _wb_healthbar _output_get)
    (else
      (bind _output_get_2 (set `/Game/InfiniteMatrix/Blueprints/BP_Player.Health` 100.0 _asbp_player))
      (`/Game/InfiniteMatrix/UI/WBP_Healthbar.UpdateHealthbar` _wb_healthbar _output_get_2)))
  (`self.K2_DestroyActor`))

(fn `UserConstructionScript`)